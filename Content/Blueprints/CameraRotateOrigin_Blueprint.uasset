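; CameraRotateOrigin is an actor that acts as a camera pivot, trailing a follow target and aiming toward the player.
; BeginPlay caches the UNAC_Player_AC and FollowTarget_Blueprint actors found in the level.
; Each Tick sets rotation to look from the follow target to the player and lerps location toward the follow target, scaled by delta time.
; Polled Q and W keys adjust a clamped vertical offset, added to pitch after the look-at.
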(event `self.ReceiveBeginPlay`
  (`|ExecutionSequence`
    (:`then_0`
      (bind _outactors (`GameplayStatics.GetAllActorsOfClass` "/Game/Blueprints/UNAC_Player_AC.UNAC_Player_AC_C"))
      (for _array_element _outactors
        (set `self.PlayerAC` _array_element)))
    (:`then_1`
      (bind _outactors_2 (`GameplayStatics.GetAllActorsOfClass` "/Game/Blueprints/FollowTarget_Blueprint.FollowTarget_Blueprint_C"))
      (for _array_element_2 _outactors_2
        (set `self.FollowTarget` _array_element_2)))))

(event `self.ReceiveTick`
  (params (DeltaSeconds :type "Float (single-precision)"))
  (bind (_returnvalue_roll _returnvalue_pitch _returnvalue_yaw) (`KismetMathLibrary.BreakRotator` (`self.K2_GetActorRotation` self)))
  (set `self.DeltaTime` DeltaSeconds)
  (`|ExecutionSequence`
    (:`then_0`
      (`self.K2_SetActorRotation` self (`KismetMathLibrary.FindLookAtRotation` (`self.K2_GetActorLocation` (`self.FollowTarget`)) (`self.K2_GetActorLocation` (`self.PlayerAC`))) false))
    (:`then_1`
      (`self.K2_SetActorLocation` self (`KismetMathLibrary.VLerp` (`self.K2_GetActorLocation` self) (`self.K2_GetActorLocation` (`self.FollowTarget`)) (* (`self.DeltaTime`) 40.0)) false false))
    (:`then_2`
      ;[1 1 1] Rotate_Camera
      (if (== (`PlayerController.GetInputAnalogKeyState` (`GameplayStatics.GetPlayerController` 0) "Q") 1.0)
        (set `self.VerticalRotation` (`KismetMathLibrary.FClamp` (+ (`self.VerticalRotation`) 1.0) -30.0 50.0))))
    (:`then_3`
      (if (== (`PlayerController.GetInputAnalogKeyState` (`GameplayStatics.GetPlayerController` 0) "W") 1.0)
        (set `self.VerticalRotation` (`KismetMathLibrary.FClamp` (- (`self.VerticalRotation`) 1.0) -30.0 50.0))))
    (:`then_4`
      (`self.K2_SetActorRotation` self (`KismetMathLibrary.MakeRotator` _returnvalue_roll (+ _returnvalue_pitch (`self.VerticalRotation`)) _returnvalue_yaw) false))))

(fn `UserConstructionScript`)