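; Main camera actor that smoothly follows a position target and faces a rotation origin.
; On BeginPlay it caches the CameraRotateOrigin, CameraPositionTarget and player AC actors by class search, keeping the last found; the player reference is unused here.
; Each Tick lerps location toward the target with delta-time-scaled alpha.
; Rotation snaps to the look-at from the target's location, rather than the camera's, to the origin.
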(event `self.ReceiveBeginPlay`
  (`|ExecutionSequence`
    (:`then_0`
      (bind _outactors (`GameplayStatics.GetAllActorsOfClass` "/Game/Blueprints/CameraRotateOrigin_Blueprint.CameraRotateOrigin_Blueprint_C"))
      (for _array_element _outactors
        (set `self.CameraRotateOrigin` _array_element)))
    (:`then_1`
      (bind _outactors_2 (`GameplayStatics.GetAllActorsOfClass` "/Game/Blueprints/CameraPositionTarget_Blueprint.CameraPositionTarget_Blueprint_C"))
      (for _array_element_2 _outactors_2
        (set `self.CameraPositionTarget` _array_element_2)))
    (:`then_2`
      (bind _outactors_3 (`GameplayStatics.GetAllActorsOfClass` "/Game/Blueprints/UNAC_Player_AC.UNAC_Player_AC_C"))
      (for _array_element_3 _outactors_3
        (set `self.PlayerAC` _array_element_3)))))

(event `self.ReceiveTick`
  (params (DeltaSeconds :type "Float (single-precision)"))
  (set `self.DeltaTime` DeltaSeconds)
  (`self.K2_SetActorLocation` self (`KismetMathLibrary.VLerp` (`self.K2_GetActorLocation` self) (`self.K2_GetActorLocation` (`self.CameraPositionTarget`)) (* 10.0 (`self.DeltaTime`))) false false)
  (`self.K2_SetActorRotation` self (`KismetMathLibrary.FindLookAtRotation` (`self.K2_GetActorLocation` (`self.CameraPositionTarget`)) (`self.K2_GetActorLocation` (`self.CameraRotateOrigin`))) false))

(fn `UserConstructionScript`)