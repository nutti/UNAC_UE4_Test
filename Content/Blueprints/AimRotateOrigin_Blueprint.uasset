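; AimRotateOrigin is an actor that repositions itself every Tick relative to the player and the follow target, apparently as an origin for aiming.
; For each UNAC_Player_AC, it snaps to that actor's location plus a fixed world-X offset.
; Inside that loop, it lerps from the snapped position toward each FollowTarget_Blueprint by a delta-time-scaled alpha, so the easing restarts from the offset each frame.
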(event `self.ReceiveTick`
  (params (DeltaSeconds :type "Float (single-precision)"))
  (bind _outactors (`GameplayStatics.GetAllActorsOfClass` "/Game/Blueprints/UNAC_Player_AC.UNAC_Player_AC_C"))
  (for _array_element _outactors
    (`self.K2_SetActorLocation` (+ (`self.K2_GetActorLocation` _array_element) (1000.0 0.0 0.0)))
    (bind _outactors_2 (`GameplayStatics.GetAllActorsOfClass` "/Game/Blueprints/FollowTarget_Blueprint.FollowTarget_Blueprint_C"))
    (for _array_element_2 _outactors_2
      (`self.K2_SetActorLocation` self (`KismetMathLibrary.VLerp` (`self.K2_GetActorLocation` self) (`self.K2_GetActorLocation` _array_element_2) (* DeltaSeconds 2.0)) false false))))

(fn `UserConstructionScript`)