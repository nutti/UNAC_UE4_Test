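; Enemy fighter actor that moves at fixed altitude and steers toward the player found at BeginPlay.
; Tick runs a state machine: pre-chase records a rough heading, rough chase turns very slowly, chase homes quickly until within range, free flies straight on a timer before restarting.
; Helper functions compare rotator differences, but the check switching rough chase to chase is unconnected, so that transition never runs.
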(event `self.ReceiveBeginPlay`
  (bind _outactors (`GameplayStatics.GetAllActorsOfClass` "/Game/Blueprints/UNAC_Player_AC.UNAC_Player_AC_C"))
  (for _array_element _outactors
    (set `self.Player` _array_element)))

(event `self.ReceiveTick`
  (params (DeltaSeconds :type "Float (single-precision)"))
  (bind (_returnvalue_x _returnvalue_y _returnvalue_z) (`KismetMathLibrary.BreakVector` (`self.K2_GetActorLocation` self)))
  (bind (_returnvalue_x_2 _returnvalue_y_2 _returnvalue_z_2) (`KismetMathLibrary.BreakVector` (`self.K2_GetActorLocation` self)))
  (bind (_returnvalue_x_3 _returnvalue_y_3 _returnvalue_z_3) (`KismetMathLibrary.BreakVector` (`self.K2_GetActorLocation` self)))
  (bind (_returnvalue_x_4 _returnvalue_y_4) (`KismetMathLibrary.BreakVector` (+ (* (`self.GetActorForwardVector` self) (* (`self.DeltaTime`) 1500.0)) (`self.K2_GetActorLocation` self))))
  (bind (_returnvalue_x_5 _returnvalue_y_5) (`KismetMathLibrary.BreakVector` (+ (* (`self.GetActorForwardVector` self) (* (`self.DeltaTime`) 1500.0)) (`self.K2_GetActorLocation` self))))
  (bind (_returnvalue_x_6 _returnvalue_y_6) (`KismetMathLibrary.BreakVector` (+ (* (`self.GetActorForwardVector` self) (* (`self.DeltaTime`) 400.0)) (`self.K2_GetActorLocation` self))))
  (set `self.DeltaTime` DeltaSeconds)
  (`|ExecutionSequence`
    (:`then_0`
      (switch `string` (`self.State`)
        (:`PRE_CHASE`
          (set `self.RoughAngle` (`KismetMathLibrary.FindLookAtRotation` (`self.K2_GetActorLocation` self) (`self.K2_GetActorLocation` (`self.Player`))))
          (set `self.State` "ROUGHLY_CHASE"))
        (:`ROUGHLY_CHASE`
          (`self.K2_SetActorRotation` (`KismetMathLibrary.RLerp` (`self.K2_GetActorRotation` self) (`self.RoughAngle`) (* (`self.DeltaTime`) 1e-05)))
          (`self.K2_SetActorLocation` (`KismetMathLibrary.MakeVector` _returnvalue_x_6 _returnvalue_y_6 _returnvalue_z_3))
          (bind _result (`self.Sub_Rotator` (`self.K2_GetActorRotation` self) (`KismetMathLibrary.FindLookAtRotation` (`self.K2_GetActorLocation` self) (`self.K2_GetActorLocation` (`self.Player`)))))
          (bind _output (`self.Abs_Rotator` _result)))
        (:`CHASE`
          (`self.K2_SetActorRotation` (`KismetMathLibrary.RLerp` (`self.K2_GetActorRotation` self) (`KismetMathLibrary.FindLookAtRotation` (`self.K2_GetActorLocation` self) (`self.K2_GetActorLocation` (`self.Player`))) (* (`self.DeltaTime`) 10.0)))
          (`self.K2_SetActorLocation` (`KismetMathLibrary.MakeVector` _returnvalue_x_4 _returnvalue_y_4 _returnvalue_z))
          (if (<= (`KismetMathLibrary.VSize2D` (- (`KismetMathLibrary.Conv_VectorToVector2D` (`self.K2_GetActorLocation` self)) (`KismetMathLibrary.Conv_VectorToVector2D` (`self.K2_GetActorLocation` (`self.Player`))))) 4000.0)
            (set `self.State` "FREE")))
        (:`FREE`
          (bind _output_get (set `self.FreeTime` (+ (`self.FreeTime`) (`self.DeltaTime`))))
          (if (>= _output_get 10.0)
            (set `self.State` "PRE_CHASE")
            (set `self.FreeTime` 0.0)
            (else
              (`self.K2_SetActorLocation` (`KismetMathLibrary.MakeVector` _returnvalue_x_5 _returnvalue_y_5 _returnvalue_z_2)))))))))

(fn `Abs_Rotator`
  (params (Input :type "Rotator Structure"))
  (returns (Output :type "Rotator Structure"))
  (return (`KismetMathLibrary.MakeRotator` (`KismetMathLibrary.Abs` Input_Roll) (`KismetMathLibrary.Abs` Input_Pitch) (`KismetMathLibrary.Abs` Input_Yaw))))

(fn `LE_Rotator`
  (params (A :type "Rotator Structure") (B :type "Rotator Structure"))
  (returns (result :type Boolean))
  (return (and (<= A_Roll B_Roll) (<= A_Pitch B_Pitch) (<= A_Yaw B_Yaw))))

(fn `Sub_Rotator`
  (params (A :type "Rotator Structure") (B :type "Rotator Structure"))
  (returns (Result :type "Rotator Structure"))
  (return (`KismetMathLibrary.MakeRotator` (- A_Roll B_Roll) (- A_Pitch B_Pitch) (- A_Yaw B_Yaw))))

(fn `UserConstructionScript`)