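; BP_Player_Bullet is a player projectile that damages what its sphere overlaps and then destroys itself.
; The overlap handler ignores player actors and other player bullets, applying damage to any other actor.
; A short lifetime counter set on BeginPlay counts down in Tick and destroys the bullet on expiry.
; BeginPlay also caches a player reference via GetAllActorsOfClass, which these graphs never read.
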(event `self.Sphere1.OnComponentBeginOverlap`
  (params (OverlappedComponent :type "PrimitiveComponent Object Reference") (OtherActor :type "Actor Object Reference") (OtherComp :type "PrimitiveComponent Object Reference") (OtherBodyIndex :type Integer) (bFromSweep :type Boolean) (SweepResult :type "HitResult Structure (by ref)"))
  (cast `/Game/Blueprints/UNAC_Player_AC` OtherActor
    (:`CastFailed`
      (cast `/Game/Blueprints/BP_Player_Bullet` OtherActor
        (:`CastFailed`
          (`GameplayStatics.ApplyDamage` OtherActor (`KismetMathLibrary.Conv_IntToDouble` (`self.Damange`)))
          (`self.K2_DestroyActor`))))))

(event `self.ReceiveTick`
  (params (DeltaSeconds :type "Float (single-precision)"))
  (bind _alivetime (`self.AliveTime`))
  (set `self.AliveTime` (- _alivetime DeltaSeconds))
  (if (<= _alivetime 0.0)
    (`self.K2_DestroyActor`)))

(event `self.ReceiveBeginPlay`
  ;[1 1 1] Initialize
  (set `self.AliveTime` 2.0)
  (bind _outactors (`GameplayStatics.GetAllActorsOfClass` "/Game/Blueprints/UNAC_Player_AC.UNAC_Player_AC_C"))
  (for _array_element _outactors
    (set `self.Player` _array_element)))

(fn `UserConstructionScript`)