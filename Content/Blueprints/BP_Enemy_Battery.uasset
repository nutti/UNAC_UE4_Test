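; BP_Enemy_Battery is a turret enemy that tracks the UNAC_Player_AC found at BeginPlay and shoots at it.
; Each tick it lerps its actor rotation toward the player at a frame-time-scaled rate.
; When a cooldown expires and signed per-axis aim differences (not absolute) are at most FireMargin, it spawns a BP_Enemy_Battery_Bullet at its Sphere's transform.
; Damage reduces AP, destroying the actor at zero or below.
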(event `self.ReceiveBeginPlay`
  ;[1 1 1] Initialize
  (bind _outactors (`GameplayStatics.GetAllActorsOfClass` "/Game/Blueprints/UNAC_Player_AC.UNAC_Player_AC_C"))
  (for _array_element _outactors
    (set `self.Player` _array_element)))

(event `self.ReceiveTick`
  (params (DeltaSeconds :type "Float (single-precision)"))
  (bind (_fire_margin_roll _fire_margin_pitch _fire_margin_yaw) (`KismetMathLibrary.BreakRotator` (`self.Fire_Margin`)))
  (bind (_returnvalue_roll _returnvalue_pitch _returnvalue_yaw) (`KismetMathLibrary.BreakRotator` (`self.K2_GetActorRotation` self)))
  (bind (_returnvalue_roll_2 _returnvalue_pitch_2 _returnvalue_yaw_2) (`KismetMathLibrary.BreakRotator` (`KismetMathLibrary.FindLookAtRotation` (`self.K2_GetActorLocation` self) (`self.K2_GetActorLocation` (`self.Player`)))))
  (`|ExecutionSequence`
    (:`then_0`
      (set `self.DeltaTime` DeltaSeconds))
    (:`then_1`
      ;[1 1 1] Move
      (`self.K2_SetActorRotation` (`KismetMathLibrary.RLerp` (`self.K2_GetActorRotation` self) (`KismetMathLibrary.FindLookAtRotation` (`self.K2_GetActorLocation` self) (`self.K2_GetActorLocation` (`self.Player`))) (* (`self.DeltaTime`) 6.0))))
    (:`then_2`
      (if (and (<= (`self.Fire_Cooltime`) 0.0) (<= (- _returnvalue_roll _returnvalue_roll_2) _fire_margin_roll) (<= (- _returnvalue_pitch _returnvalue_pitch_2) _fire_margin_pitch) (<= (- _returnvalue_yaw _returnvalue_yaw_2) _fire_margin_yaw))
        (set `self.Fire_Cooltime` 2.0)
        (`|SpawnActorFromClass` "/Game/Blueprints/BP_Enemy_Battery_Bullet.BP_Enemy_Battery_Bullet_C" (`SceneComponent.K2_GetComponentToWorld` (`self.Sphere`)) "Undefined" "OverrideRootScale")))
    (:`then_3`
      (set `self.Fire_Cooltime` (- (`self.Fire_Cooltime`) (`self.DeltaTime`))))))

(event `self.ReceiveAnyDamage`
  (params (Damage :type "Float (single-precision)") (DamageType :type "DamageType Object Reference") (InstigatedBy :type "Controller Object Reference") (DamageCauser :type "Actor Object Reference"))
  ;[1 1 1] Damage
  (set `self.AP` (- (`self.AP`) (`KismetMathLibrary.FTrunc` Damage)))
  (if (<= (`self.AP`) 0)
    (`self.K2_DestroyActor`)))

(fn `UserConstructionScript`)