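; Player actor with boosters, driven by physics on its Cube component from keys polled on player controller 0.
; Tick adds boost force (upward or forward-and-up), yaw torque and directional quick-boost force.
; The quick-boost cooldown restarts even with zero force, so boosts land only on periodic ticks.
; An older velocity-based movement chain with custom gravity and drag is disconnected, though Hit still edits its PlayerVelocity.
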(event `self.ReceiveTick`
  (params (DeltaSeconds :type "Float (single-precision)"))
  (bind _returnvalue (`GameplayStatics.GetPlayerController` 0))
  (bind _returnvalue_2 (/ (`self.Booster_Force`) 2.0))
  (bind (_returnvalue_x _returnvalue_y _returnvalue_z) (`KismetMathLibrary.BreakVector` (* (`SceneComponent.GetForwardVector` (`self.Cube`)) _returnvalue_2)))
  (set `self.Delta_Time` DeltaSeconds)
  (`|ExecutionSequence`
    (:`then_0`
      ;[1 1 1] Booster_Phys
      (if (== (`PlayerController.GetInputAnalogKeyState` (`GameplayStatics.GetPlayerController` 0) "Z") 1.0)
        (if (== (`PlayerController.GetInputAnalogKeyState` (`GameplayStatics.GetPlayerController` 0) "Up") 1.0)
          (`PrimitiveComponent.AddForce` (`self.Cube`) (`KismetMathLibrary.MakeVector` _returnvalue_x _returnvalue_y (+ _returnvalue_z _returnvalue_2)) "None" false)
          (else
            (`PrimitiveComponent.AddForce` (`self.Cube`) (`KismetMathLibrary.MakeVector` 0.0 0.0 (`self.Booster_Force`)) "None" false)))))
    (:`then_1`
      ;[1 1 1] Rotate_Phys
      (`|ExecutionSequence`
        (:`then_0`
          (if (== (`PlayerController.GetInputAnalogKeyState` (`GameplayStatics.GetPlayerController` 0) "Left") 1.0)
            (`PrimitiveComponent.AddTorque` (`self.Cube`) (`KismetMathLibrary.MakeVector` 0.0 0.0 (* (`self.Rotate_Torque`) -1.0)) "None" false)
            (elif (== (`PlayerController.GetInputAnalogKeyState` (`GameplayStatics.GetPlayerController` 0) "Right") 1.0)
              (`PrimitiveComponent.AddTorque` (`self.Cube`) (`KismetMathLibrary.MakeVector` 0.0 0.0 (`self.Rotate_Torque`)) "None" false))))))
    (:`then_2`
      ;[1 1 1] Quick_Booster_Phys
      (`|ExecutionSequence`
        (:`then_0`
          (set `self.QB_Force` (0.0 0.0 0.0)))
        (:`then_1`
          (if (== (`PlayerController.GetInputAnalogKeyState` _returnvalue "S") 1.0)
            (set `self.QB_Force` (* (`SceneComponent.GetRightVector` (`self.Cube`)) (`self.QB_Force_Magnitude`)))))
        (:`then_2`
          (if (== (`PlayerController.GetInputAnalogKeyState` _returnvalue "A") 1.0)
            (set `self.QB_Force` (* (`SceneComponent.GetRightVector` (`self.Cube`)) (* (`self.QB_Force_Magnitude`) -1.0)))))
        (:`then_3`
          (if (== (`PlayerController.GetInputAnalogKeyState` _returnvalue "X") 1.0)
            (set `self.QB_Force` (* (`SceneComponent.GetForwardVector` (`self.Cube`)) (`self.QB_Force_Magnitude`)))))
        (:`then_4`
          (if (== (`PlayerController.GetInputAnalogKeyState` _returnvalue "Down") 1.0)
            (set `self.QB_Force` (* (`SceneComponent.GetForwardVector` (`self.Cube`)) (* (`self.QB_Force_Magnitude`) -1.0)))))
        (:`then_5`
          (`self.QuickBooster_Phys` 0.4 (`self.Delta_Time`) (`self.QB_Force`) (`self.Cube`)))))))

(event `self.ReceiveHit`
  (params (MyComp :type "PrimitiveComponent Object Reference") (Other :type "Actor Object Reference") (OtherComp :type "PrimitiveComponent Object Reference") (bSelfMoved :type Boolean) (HitLocation :type "Vector Structure") (HitNormal :type "Vector Structure") (NormalImpulse :type "Vector Structure") (Hit :type "HitResult Structure (by ref)"))
  ;[1 1 1] Collision
  (if (and (== MyComp (`self.Cube`)) true)
    (bind _implus (`self.GetImplus` HitNormal))
    (set `self.PlayerVelocity` (* _implus (`self.PlayerVelocity`)))))

(fn `ApplyAirResistance`
  (params (input :type "Vector Structure") (resistance :type "Float (double-precision)") (mass :type "Float (double-precision)") (deltaTime :type "Float (double-precision)"))
  (returns (output :type "Vector Structure"))
  (return (* input (`KismetMathLibrary.MultiplyMultiply_FloatFloat` 2.71 (* (/ resistance mass) -1.0 deltaTime)))))

(fn `ApplyGravity`
  (params (input :type "Vector Structure") (gravity :type "Vector Structure") (deltaTime :type "Float (double-precision)"))
  (returns (out :type "Vector Structure"))
  (return (+ (* gravity deltaTime) input)))

(fn `GetImplus`
  (params (normal :type "Vector Structure"))
  (returns (Implus :type "Vector Structure"))
  (return (- (1.0 1.0 1.0) normal)))

(fn `QuickBooster`
  (params (Fire :type Boolean) (CoolTime :type "Float (double-precision)") (DeltaTime :type "Float (double-precision)") (Input :type "Vector Structure") (QB_Velocity :type "Vector Structure"))
  (returns (Output :type "Vector Structure"))
  (bind _output_get (set `self.QB_CooolTime` (- (`self.QB_CooolTime`) DeltaTime)))
  (`KismetSystemLibrary.PrintString` (`KismetStringLibrary.Conv_DoubleToString` _output_get) true true (struct :`G` 0.66 :`B` 1.0 :`A` 1.0) 0.0)
  (if (and (== Fire true) (<= (`self.QB_CooolTime`) 0.0))
    (set `self.QB_CooolTime` CoolTime)
    (return (+ Input QB_Velocity))
    (else
      (return Input))))

(fn `QuickBooster_Phys`
  (params (`Cool TIme` :type "Float (double-precision)") (`Delta Time` :type "Float (double-precision)") (Force :type "Vector Structure") (Target :type "PrimitiveComponent Object Reference"))
  (set `self.QB_CooolTime` (- (`self.QB_CooolTime`) `Delta Time`))
  (if (<= (`self.QB_CooolTime`) 0.0)
    (`PrimitiveComponent.AddForce` Target Force "None" false)
    (set `self.QB_CooolTime` `Cool TIme`)))

(fn `UpdateLocation`
  (params (velocity :type "Vector Structure") (actor :type "Actor Object Reference"))
  (`self.K2_SetActorLocation` actor (+ velocity (`self.K2_GetActorLocation` actor)) false false)
  (return))

(fn `UserConstructionScript`)