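; BP_Enemy_Battery_Bullet is the projectile actor for the battery enemy, damaging what it hits.
; When Sphere1 begins an overlap, it ignores battery enemies and other battery bullets, applies Damage to any other actor, then destroys itself.
; Tick counts AliveTime down by delta seconds and destroys the bullet once it runs out.
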(event `self.Sphere1.OnComponentBeginOverlap`
  (params (OverlappedComponent :type "PrimitiveComponent Object Reference") (OtherActor :type "Actor Object Reference") (OtherComp :type "PrimitiveComponent Object Reference") (OtherBodyIndex :type Integer) (bFromSweep :type Boolean) (SweepResult :type "HitResult Structure (by ref)"))
  (cast `/Game/Blueprints/BP_Enemy_Battery` OtherActor
    (:`CastFailed`
      (cast `/Game/Blueprints/BP_Enemy_Battery_Bullet` OtherActor
        (:`CastFailed`
          (`GameplayStatics.ApplyDamage` OtherActor (`KismetMathLibrary.Conv_IntToDouble` (`self.Damage`)))
          (`self.K2_DestroyActor`))))))

(event `self.ReceiveTick`
  (params (DeltaSeconds :type "Float (single-precision)"))
  (bind _alivetime (`self.AliveTime`))
  (set `self.AliveTime` (- _alivetime DeltaSeconds))
  (if (<= _alivetime 0.0)
    (`self.K2_DestroyActor`)))

(fn `UserConstructionScript`)